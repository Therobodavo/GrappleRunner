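; GrappleRunnerCharacter4 is a runner character Blueprint that handles sideways switching between three lanes.
; A and D step the target lane down or up, clamped to the valid range, and restart a shared timeline.
; The timeline lerps the actor's Y between stored lane positions while keeping the capsule's X and Z, then commits the new lane when finished.
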(event `Key|A`
  (params (Key :type "Key Structure"))
  (bind _laney (`self.LaneY`))
  (bind (_returnvalue_x _returnvalue_y _returnvalue_z) (`KismetMathLibrary.BreakVector` (`SceneComponent.K2_GetComponentLocation` (`self.CapsuleComponent`))))
  (:`Pressed`
    (set `self.NewLane` (`KismetMathLibrary.Clamp` (+ (`self.Lane`) -1) 0 2))
    (bind (_direction _lane_y) (`Timeline|LerpTimeline` :!via `PlayFromStart` :!label _label)
      (:`Update`
        (`self.K2_SetActorLocation` (`KismetMathLibrary.MakeVector` _returnvalue_x (`KismetMathLibrary.Lerp` (`|GetArrayItem` _laney (`self.Lane`)) (`|GetArrayItem` _laney (`self.NewLane`)) _lane_y) _returnvalue_z)))
      (:`Finished`
        (set `self.Lane` (`self.NewLane`))))))

(event `Key|D`
  (params (Key :type "Key Structure"))
  (:`Pressed`
    (set `self.NewLane` (`KismetMathLibrary.Clamp` (+ (`self.Lane`) 1) 0 2))
    (goto _label :!via `PlayFromStart`)))

(fn `UserConstructionScript`)