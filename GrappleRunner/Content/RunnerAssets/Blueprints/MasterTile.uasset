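; MasterTile is a track tile for an endless runner that places pipe obstacles and extends the track.
; On BeginPlay, nested coin flips spawn pipes at three lane points, so each lane gets one only if the previous lane did.
; When the ThirdPersonCharacter overlaps its Box, the game mode spawns another tile and this one destroys itself after a short delay.
; The spawned pipes are not destroyed here.
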(event `self.ReceiveBeginPlay`
  (`self.Spawn Obstacles`))

(event `self.ReceiveTick`
  (params (DeltaSeconds :type "Float (single-precision)")))

(event `self.Box.OnComponentBeginOverlap`
  (params (OverlappedComponent :type "PrimitiveComponent Object Reference") (OtherActor :type "Actor Object Reference") (OtherComp :type "PrimitiveComponent Object Reference") (OtherBodyIndex :type Integer) (bFromSweep :type Boolean) (SweepResult :type "HitResult Structure (by ref)"))
  (cast `/Game/ThirdPersonCPP/Blueprints/ThirdPersonCharacter` OtherActor)
  (bind _asmy_grapple_runner_game_mode (cast `/Game/RunnerAssets/Blueprints/MyGrappleRunnerGameMode` (`GameplayStatics.GetGameMode`)))
  (`/Game/RunnerAssets/Blueprints/MyGrappleRunnerGameMode.SpawnTile` _asmy_grapple_runner_game_mode)
  (`KismetSystemLibrary.Delay` 0.5)
  (`self.K2_DestroyActor`))

(fn `Spawn Obstacles`
  (switch `int` (`KismetMathLibrary.RandomIntegerInRange` 0 1)
    (:`1`
      (`|SpawnActorFromClass` "/Game/RunnerAssets/Blueprints/Obstacles_pipe.Obstacles_pipe_C" (`SceneComponent.K2_GetComponentToWorld` (`self.Lane0`)) "Undefined" "OverrideRootScale" null null)
      (switch `int` (`KismetMathLibrary.RandomIntegerInRange` 0 1)
        (:`1`
          (`|SpawnActorFromClass` "/Game/RunnerAssets/Blueprints/Obstacles_pipe.Obstacles_pipe_C" (`SceneComponent.K2_GetComponentToWorld` (`self.Lane1`)) "Undefined" "OverrideRootScale" null null)
          (switch `int` (`KismetMathLibrary.RandomIntegerInRange` 0 1)
            (:`1`
              (`|SpawnActorFromClass` "/Game/RunnerAssets/Blueprints/Obstacles_pipe.Obstacles_pipe_C" (`SceneComponent.K2_GetComponentToWorld` (`self.Lane2`)) "Undefined" "OverrideRootScale" null null))))))))

(fn `UserConstructionScript`)